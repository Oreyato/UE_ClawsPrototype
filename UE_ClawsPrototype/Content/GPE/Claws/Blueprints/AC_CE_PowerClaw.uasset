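; Power claw component: a one-shot claw ability that powers enemies and other powerable objects in front of its owner.
; BeginPlay caches range and effects from the claw data asset, plus the player's claw meshes.
; ActivateClaw plays animation, slash Niagara and Wwise audio, then line-traces in a direction signed by claw side.
; BPI_Enemy or BPI_WetPowered hits receive powered messages and knock the player back; ResetClaw re-arms it.
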(event `self.ReceiveBeginPlay`
  (bind _datas (`self.Datas`))
  (`parent.ReceiveBeginPlay`)
  (set `self.Range` (`/Game/GPE/Claws/Data/PDA_PowerClaw.Range` _datas))
  (set `self.Hit Effect` (`/Game/GPE/Claws/Data/PDA_PowerClaw.HitEffect` _datas))
  (set `self.Slash Effect` (`/Game/GPE/Claws/Data/PDA_PowerClaw.SlashEffect` _datas))
  (bind _asbp_chara_base (cast `/Game/Setup/Remi/BP_CharaBase` (`GameplayStatics.GetPlayerCharacter` 0)))
  (bind _output_get (set `self.PlayerCharacter` _asbp_chara_base))
  ;[0.6588 0.2275 0.9294] TEMPORARY
  (set `self.SK Left Claw` (`/Game/Setup/Remi/BP_CharaBase.SK_LeftClaw` _output_get))
  (set `self.SK Right Claw` (`/Game/Setup/Remi/BP_CharaBase.SK_RightClaw` _output_get)))

(fn `ActivateClaw`
  (params (`Common Parameters` :type "/Game/GPE/Claws/Blueprints/SCommonClawActivationParameters Structure"))
  (locals (RayRange :type "Float (double-precision)") (HitLocation :type "Vector Structure" :default (0.0 0.0 0.0)) (Direction :type "Float (double-precision)") (MechanismSocketLocation :type "Vector Structure" :default (0.0 0.0 0.0)) (Orientation :type "Rotator Structure") (SlashNS :type "NiagaraComponent Object Reference"))
  (bind _playercharacter (`self.PlayerCharacter`))
  (bind _slashns (`local.SlashNS`))
  (bind (_x _y _z) (`KismetMathLibrary.BreakVector3f` (`local.HitLocation`)))
  (if (not (`self.bUsedOnce`))
    (set `self.bUsedOnce` true)
    (bind _output_get (set `self.IsRightClaw` `Common Parameters_bIsRightClaw_7_D13CA49743B6B60F33DA7B8821A3BDF5`))
    (if _output_get
      (set `local.Direction` 1.0)
      (set `local.SlashNS` (`/Game/Setup/Remi/BP_CharaBase.NS_LeftClawMechanism` _playercharacter))
      (set `local.Orientation` (struct :`Yaw` 180.0))
      (else
        (set `local.Direction` -1.0)
        (set `local.SlashNS` (`/Game/Setup/Remi/BP_CharaBase.NS_RightClawMechanism` _playercharacter))
        (set `local.Orientation` (struct))))
    (set `local.RayRange` (* (`self.Range`) (`local.Direction`)))
    ;[1 1 1] Play a first animation even if the claw doesn't hit anything
    (`NiagaraComponent.SetAsset` _slashns (`self.Slash Effect`) true)
    (`NiagaraComponent.ResetSystem` _slashns)
    (`SkeletalMeshComponent.PlayAnimation` (`self.SK Left Claw`) "/Game/ART_GPE/CLAWS/POWERCLAW/POWERCLAW_Anims/AM_PowerClaw_Activate.AM_PowerClaw_Activate" false)
    (`SkeletalMeshComponent.PlayAnimation` (`self.SK Right Claw`) "/Game/ART_GPE/CLAWS/POWERCLAW/POWERCLAW_Anims/AM_PowerClaw_Activate.AM_PowerClaw_Activate" false) ; ???
    (`AkGameplayStatics.PostEventAtLocation` "/Game/WwiseAudio/Play_Powerclaw_Deploying.Play_Powerclaw_Deploying" (`Actor.K2_GetActorLocation` (`self.PlayerCharacter`)))
    (bind _outhit (`/Game/Utilities/BPFL.Forward Line Trace` (`self.GetOwner`) (`local.RayRange`) (`|MakeArray` (`GameplayStatics.GetPlayerCharacter` 0) :!type "Actor Object Reference")))
    (bind (_bblockinghit _binitialoverlap _time _distance _location _impactpoint _normal _impactnormal _physmat _hitactor) (`GameplayStatics.BreakHitResult` _outhit))
    (if _bblockinghit
      (set `local.HitLocation` _impactpoint)
      (set `self.Hit Actor` _hitactor)
      ;[1 1 1] When the trace hits something do:
      ;;[0.6588 0.2275 0.9294] Will be removed
      (if (`KismetSystemLibrary.DoesImplementInterface` (`self.Hit Actor`) "/Game/Interfaces/BPI_Enemy.BPI_Enemy_C")
        ;;;[1 1 1] Hit Enemy
        (message `/Game/Interfaces/BPI_Enemy.Powered` (`self.Hit Actor`))
        (`AkGameplayStatics.PostEventAtLocation` "/Game/WwiseAudio/Events/Default_Work_Unit/Play_Hit_Success.Play_Hit_Success" (`Actor.K2_GetActorLocation` (`self.PlayerCharacter`)) :!label _label)
        (`/Game/Setup/Remi/BP_CharaBase.KnockBack` (`self.PlayerCharacter`))
        (`NiagaraFunctionLibrary.SpawnSystemAtLocation` (`self.Hit Effect`) (`KismetMathLibrary.MakeVector` _x _y (+ _z 25.0)) (struct) (5.0 5.0 5.0))
        (else
          ;;[1 1 1] Hit something else that can be powered
          (if (`KismetSystemLibrary.DoesImplementInterface` (`self.Hit Actor`) "/Game/Interfaces/BPI_WetPowered.BPI_WetPowered_C")
            (message `/Game/Interfaces/BPI_WetPowered.GetPowered` (`self.Hit Actor`) (`local.HitLocation`))
            (goto _label)
            (else
              (`AkGameplayStatics.PostEventAtLocation` "/Game/WwiseAudio/Events/Default_Work_Unit/Play_Hit_Fail.Play_Hit_Fail" (`Actor.K2_GetActorLocation` (`self.PlayerCharacter`)))))))
      (else
        ;[1 1 1] Hit none of them: failed
        (`AkGameplayStatics.PostEventAtLocation` "/Game/WwiseAudio/Events/Default_Work_Unit/Play_Hit_Nothing.Play_Hit_Nothing" (`Actor.K2_GetActorLocation` (`self.PlayerCharacter`)))
        (`NiagaraFunctionLibrary.SpawnSystemAtLocation` "/Game/ART_Vfx/Niagara/Systeme/Abilities/NS_PowerClaw_Sparks.NS_PowerClaw_Sparks" (`local.HitLocation`))))))

(fn `DetectionLineTrace`
  (params (Range :type "Float (double-precision)") (ActorsToIgnore :type "Array of Actor Object Reference (by ref)"))
  (returns (OutHit :type "HitResult Structure"))
  (return))

(fn `GetPDAClaw`
  (returns (`PDA Claw` :type "/Game/GPE/Claws/Data/PDA_Claw Object Reference"))
  (return (`self.Datas`)))

(fn `ResetClaw`
  (set `self.bUsedOnce` false))